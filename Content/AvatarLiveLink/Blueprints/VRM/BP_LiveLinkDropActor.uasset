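; Live Link avatar actor that loads dropped VRM files at runtime and swaps them onto the BP_VRMTest player pawn.
; VrmDropFiles triggers an async load with extension-based scale, then a dispatcher passes the asset list to ApplyVrm.
; ApplyVrm replaces the spawned MToonActor, attaches it to the pawn and uses VrmAnimInstanceCopy to mirror the pawn's source skeleton.
; If a child actor exists, it also moves the camera spring arm to the head socket.
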(event Custom|LoadVrmFromFilePath
  (params (FileName :type String))
  ;[1 1 1] VRMLoad & Apply
  (Utilities|FlowControl|Sequence
    (:then_1
      (bind _outputpin (Utilities|LoadVrm FileName))
      (Default|CallOnApplyNewVRM _outputpin))))

(event Custom|ApplyVrmFromAssetList
  (params (VRMAssetList :type Vrm%20Asset%20List%20Object%20Object%20Reference))
  ;[1 1 1] BindEvent ApplyVRM
  (CallFunction|ApplyVrm VRMAssetList))

(event EventBeginPlay
  (Utilities|FlowControl|Sequence
    (:then_1
      ;[1 1 1] BindEvent ApplyVRM
      (EventDispatchers|BindEventtoOnApplyNewVRM (delegate Custom|ApplyVrmFromAssetList)))
    (:then_2
      ;[1 1 1] VRMLoad & Apply
      (EventDispatchers|AssignOnDropFiles (Variables|Default|GetVrmDropFiles) (delegate Custom|LoadVrmFromFilePath)))))

(fn ConstructionScript)

(fn ApplyVrm
  (params (VRMAssetList :type Vrm%20Asset%20List%20Object%20Object%20Reference))
  (bind _returnvalue (Game|Player|GetPlayerPawn 0))
  (bind _asbp_vrmtest (Utilities|Casting|CastToBP_VRMTest _returnvalue))
  (bind _skeletalmeshsrc (Variables|/Game/AvatarLiveLink/Blueprints/BP_VRMTest.BP_VRMTest_C|GetSkeletalMeshSrc _asbp_vrmtest))
  (Utilities|FlowControl|Sequence
    (:then_0
      (bind _spawnedactor (Variables|Default|GetSpawnedActor)
        (:then
          (Actor|DestroyActor _spawnedactor))
        (:else)))
    (:then_1
      (bind _returnvalue_2 (Game|SpawnActorfromClass "/VRM4U/Util/Actor/MToonActor.MToonActor_C" (Transformation|GetActorTransform) "Undefined" 0 VRMAssetList 5e+02 false true 0 false 0 0))
      (bind _output_get (Variables|Default|SetSpawnedActor _returnvalue_2))
      (Utilities|FlowControl|Sequence
        (:then_0
          (Class|SkeletalMeshComponent|SetAnimClass (Variables|/VRM4U/Util/Actor/MToonActor.MToonActor_C|GetSkeletalMesh _returnvalue_2) "/Script/VRM4U.VrmAnimInstanceCopy")
          (bind _asvrm_anim_instance_copy (Utilities|Casting|CastToVrmAnimInstanceCopy (Components|SkeletalMesh|GetAnimInstance (Variables|/VRM4U/Util/Actor/MToonActor.MToonActor_C|GetSkeletalMesh _returnvalue_2))))
          (Class|VrmAnimInstanceCopy|SetSkeletalMeshCopyData _asvrm_anim_instance_copy VRMAssetList _skeletalmeshsrc 0 "/VRM4U/Util/BaseCharacter/Mesh/VRoidSimple_VrmAssetList.VRoidSimple_VrmAssetList")
          (Transformation|AttachActorToActor _returnvalue_2 _asbp_vrmtest "None" "SnapToTarget" "SnapToTarget" "SnapToTarget" true)
          (Transformation|AttachComponentToComponent (Variables|/VRM4U/Util/Actor/MToonActor.MToonActor_C|GetSkeletalMesh _returnvalue_2) _skeletalmeshsrc "None" "SnapToTarget" "SnapToTarget" "SnapToTarget" true))
        (:then_1
          (bind _childactor (Variables|/VRM4U/Util/Actor/MToonActor.MToonActor_C|GetChildActor _output_get)
            (:then
              (Utilities|FlowControl|Sequence
                (:then_0
                  (bind _childactor_2 (Variables|/Script/Engine.ChildActorComponent|GetChildActor _childactor)
                    (:then
                      (Actor|DestroyActor _childactor_2))
                    (:else)))
                (:then_2
                  (Components|DestroyComponent _skeletalmeshsrc))
                (:then_3
                  (Rendering|SetVisibility _skeletalmeshsrc false false))
                (:then_4
                  ;[1 1 1] AdjustLockAtCamera
                  (bind _array_element (Utilities|Array|ForEachLoopwithBreak (Transformation|GetAllSocketNames (Variables|/VRM4U/Util/Actor/MToonActor.MToonActor_C|GetSkeletalMesh (Variables|Default|GetSpawnedActor))) :!label _label)
                    (:LoopBody
                      (LocalVariables|Setheadsocket _array_element)
                      (LocalVariables|SetisFind (Class|KismetStringLibrary|MatchesWildcard (Utilities|String|ToString(Name) _array_element) "*head" "IgnoreCase"))
                      (if (Class|KismetStringLibrary|MatchesWildcard (Utilities|String|ToString(Name) _array_element) "*head" "IgnoreCase")
                        (goto _label Break)))
                    (:Completed
                      (if (LocalVariables|GetisFind)
                        (bind _springarm (Class|BPIBasicPlayerCharacter|GetSpringArm(Message) (Game|Player|GetPlayerPawn 0)))
                        (Transformation|SetRelativeLocation _springarm (Math|Transform|InverseTransformLocation (Transformation|GetActorTransform (Variables|Default|GetSpawnedActor)) (Transformation|GetSocketLocation (Variables|/VRM4U/Util/Actor/MToonActor.MToonActor_C|GetSkeletalMesh (Variables|Default|GetSpawnedActor)) (LocalVariables|Getheadsocket))) true false)))))))
            (:else)))))))