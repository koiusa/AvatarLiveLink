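; Actor component that gives access to a runtime VRM avatar for its owner, exposing attachment state and hand bone data.
; FindVRMActor searches the owner's directly attached actors for the first MToonActor, and IsAttached reports whether one is found.
; Hand queries instead go through player controller 0 messages for bone names and the spawned actor, whose skeletal mesh supplies world-space hand transforms.
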(fn GetHandTransform
  (bind _returnvalue (Game|GetPlayerController 0))
  (Utilities|FlowControl|Sequence
    (:then_0
      (bind _spawnedactor (Class|BPIVRMRuntimeController|GetSpawnedActor(Message) _returnvalue))
      (LocalVariables|SetSpawnedActor _spawnedactor))
    (:then_1
      (bind _bonename (Class|BPIVRMRuntimeController|GetBoneName(Message) _returnvalue "NewEnumerator1"))
      (LocalVariables|SetLHand (Transformation|GetSocketTransform (Variables|/VRM4U/Util/Actor/MToonActor.MToonActor_C|GetSkeletalMesh (LocalVariables|GetSpawnedActor)) _bonename "RTS_World")))
    (:then_2
      (bind _bonename_2 (Class|BPIVRMRuntimeController|GetBoneName(Message) _returnvalue "NewEnumerator2"))
      (LocalVariables|SetRHand (Transformation|GetSocketTransform (Variables|/VRM4U/Util/Actor/MToonActor.MToonActor_C|GetSkeletalMesh (LocalVariables|GetSpawnedActor)) _bonename_2 "RTS_World")))
    (:then_3
      (return (LocalVariables|GetLHand) (LocalVariables|GetRHand)))))

(fn IsAttached
  (bind _isfind (CallFunction|FindVRMActor))
  (return _isfind))

(fn FindVRMActor
  (bind _returnvalue (Components|GetOwner))
  (bind _outactors (Actor|GetAttachedActors _returnvalue true false))
  (if (> (Utilities|Array|Length _outactors) 0)
    (bind _array_element (Utilities|Array|ForEachLoopwithBreak _outactors :!label _label)
      (:LoopBody
        (bind _asmtoon_actor (Utilities|Casting|CastToMToonActor _array_element))
        (LocalVariables|SetVRMActor _asmtoon_actor)
        (LocalVariables|SetIsFind? true)
        (goto _label Break))
      (:Completed
        (return (LocalVariables|GetVRMActor) (LocalVariables|GetIsFind?))))
    (else
      (return 0 false))))

(fn GetHandBoneNmae
  (bind _returnvalue (Game|GetPlayerController 0))
  (Utilities|FlowControl|Sequence
    (:then_0
      (bind _bonename (Class|BPIVRMRuntimeController|GetBoneName(Message) _returnvalue "NewEnumerator1")))
    (:then_1
      (bind _bonename_2 (Class|BPIVRMRuntimeController|GetBoneName(Message) _returnvalue "NewEnumerator2")))
    (:then_2
      (return _bonename _bonename_2))))