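; Blueprint function library of VRM helpers for AvatarLiveLink: showing the open-VRM UI and importing a VRM avatar at runtime.
; ApplyWidget adds the WB_LiveLinkOpenVRM widget to the player's screen and shows the mouse cursor.
; LoadVRMFromFilePath gets the runtime loader from player controller 0 through a message call and opens a file dialog.
; When a file is chosen, it sets the import material type and loads that file.
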(fn ApplyWidget
  (params (PlayerController :type Player%20Controller%20Object%20Reference))
  ;[1 1 1] Create Widget
  (bind _returnvalue (UserInterface|CreateWidget "/Game/AvatarLiveLink/Blueprints/VRM/WB_LiveLinkOpenVRM.WB_LiveLinkOpenVRM_C" PlayerController))
  (UserInterface|Viewport|AddtoPlayerScreen _returnvalue)
  (Variables|/Script/Engine.PlayerController|SetbShowMouseCursor PlayerController true))

(fn LoadVRMfromFilePath
  (params (MaterialType :type EVRMImportMaterialType%20Enum :default "VRMIMT_Auto"))
  (bind _vrmloader (Class|BPIVRMRuntimeController|GetVRMLoader(Message) (Game|GetPlayerController 0)))
  (bind _output_get (LocalVariables|SetVRMRuntimeLoader _vrmloader))
  (bind (_filename _returnvalue) (Class|VrmDropFilesComponent|VRMGetOpenFileName (Variables|/Game/AvatarLiveLink/Blueprints/VRM/BPC_VRMRuntimeLoader.BPC_VRMRuntimeLoader_C|GetVrmDropFiles _output_get)))
  (if _returnvalue
    (Utilities|Struct|SetmembersinImportOptionData (Variables|/Game/AvatarLiveLink/Blueprints/VRM/BPC_VRMRuntimeLoader.BPC_VRMRuntimeLoader_C|GetImportOption _output_get) MaterialType)
    (Default|LoadVrmfromFilePath (LocalVariables|GetVRMRuntimeLoader) _filename)))