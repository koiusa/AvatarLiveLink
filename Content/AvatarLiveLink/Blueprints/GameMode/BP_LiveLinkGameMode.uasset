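; Game mode for the LiveLink avatar game that spawns player robots at a spawn pad.
; GetActiveSpawnPoint returns the cached pad or searches all BP_SpawnPoint actors, caching the first found and printing an error if none exists.
; Comments describe an IsStartSpawnPad check, but the loop condition is always true.
; SpawnPlayer delegates spawning to that pad with the source character and controller, then prints and returns the result.
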(fn ConstructionScript)

(fn GetActiveSpawnPoint
  ;[0.4592 1 0.9141] Try to find a spawn pad to spawn our robots.
  ;;[0.7115 1 0.9541 1 12] Do we have a valid reference. Then take that!
  (Variables|Default|GetActiveSpawnPoint
    (:then
      (return (Variables|Default|GetActiveSpawnPoint)))
    (:else
      ;;[0.7115 1 0.9541 1 12] If not, we check all actors in the scene. If that has the bool IsStartSpawnPad set to true, we save that as active. (if more than one has it set, the last in that list will be taken here)
      (bind _outactors (Actor|GetAllActorsOfClass "/Game/AvatarLiveLink/Blueprints/BP_SpawnPoint.BP_SpawnPoint_C"))
      (bind _array_element (Utilities|Array|ForEachLoopwithBreak _outactors :!label _label)
        (:LoopBody
          (if true
            (Variables|Default|SetActiveSpawnPoint _array_element)
            (goto _label Break)))
        (:Completed
          ;;[0.7115 1 0.9541 1 12] If we found one, we take that, if not...
          (Utilities|IsValid (Variables|Default|GetActiveSpawnPoint)
            (:Is%20Valid
              (return (Variables|Default|GetActiveSpawnPoint)))
            (:Is%20Not%20Valid
              ;;[0.7115 1 0.9541 1 12] If not we take the first one in the list, if there is none...
              (Utilities|IsValid (Utilities|Array|Get(acopy) _outactors)
                (:Is%20Valid
                  (Variables|Default|SetActiveSpawnPoint 0)
                  (return (Variables|Default|GetActiveSpawnPoint)))
                (:Is%20Not%20Valid
                  ;;[0.7115 1 0.9541 1 12] We complain. The game will not be playable.
                  (Development|PrintString "No Spawnpad found!"))))))))))

(fn SpawnPlayer
  (params (SourceCharacter :type Character%20Class%20Reference) (PlayerController :type Controller%20Object%20Reference))
  (bind _character (Default|SpawnPlayer (Spawn|GetActiveSpawnPoint) SourceCharacter PlayerController))
  (Development|PrintString (Utilities|GetDisplayName _character))
  (return _character))