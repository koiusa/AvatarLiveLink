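; Actor component that plays footstep audio for its owning actor, varying with movement speed and floor surface.
; On BeginPlay it adds an audio component to the owner and bundles it with settings and surface lookup into an adapter struct.
; PlaySound scales volume by owner speed, line-traces downward for the physical material, and passes play, volume and floor parameters to the sound before playing it.
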(event Custom|Initialize
  (bind _returnvalue (Game|AddComponentbyClass (Components|GetOwner) "/Script/Engine.AudioComponent" false))
  (Variables|Default|SetFootSteps _returnvalue)
  (Audio|Components|Audio|SetSound (Variables|Default|GetFootSteps) (Variables|Components|GetSoundSource))
  (Variables|Default|SetFootStepsAdapterData (Utilities|Struct|MakeFootStepsAdapterData (Variables|Default|GetFootSteps) true 1.0 (Variables|Default|GetSurface))))

(event EventBeginPlay
  (CallFunction|Initialize))

(fn CurrentStepsData
  (return (Variables|Default|GetFootStepsAdapterData)))

(fn PlaySound
  (bind _returnvalue (Components|GetOwner))
  (bind _returnvalue_2 (Transformation|GetActorLocation _returnvalue))
  (bind _adapterdata (CallFunction|CurrentStepsData))
  (LocalVariables|SetFootStepAudio (.FootStepAudio (Utilities|Struct|BreakFootStepsAdapterData _adapterdata)))
  (Utilities|FlowControl|Sequence
    (:then_0
      ;[1 1 1] GetSpeed
      (LocalVariables|SetSpeed (Math|Vector|VectorLength (Transformation|GetVelocity (Components|GetOwner)))))
    (:then_1
      ;[1 1 1] SetParameter
      (Effects|Components|ParticleSystem|SetBoolParameter (LocalVariables|GetFootStepAudio) "step_play" (.IsFootStepsPlay (Utilities|Struct|BreakFootStepsAdapterData _adapterdata)))
      (Audio|Parameter|SetFloatParameter (LocalVariables|GetFootStepAudio) "step_volume" (* (.FootStepsVolume (Utilities|Struct|BreakFootStepsAdapterData _adapterdata)) (Math|Float|MapRangeClamped (LocalVariables|GetSpeed) 2e+02 6e+02 0.55 1.0)) :!class /Script/Engine.AudioComponent))
    (:then_2
      ;[1 1 1] Type of Floor
      (bind _outhit (Collision|LineTraceByChannel _returnvalue_2 (- _returnvalue_2 "0, 0,150.000000") "TraceTypeQuery1" false 0 "None"))
      (Effects|Components|ParticleSystem|SetIntParameter (LocalVariables|GetFootStepAudio) "floor" (Utilities|Array|FindItem (.Surface (Utilities|Struct|BreakFootStepsAdapterData _adapterdata)) (.PhysMat (Collision|BreakHitResult _outhit)))))
    (:then_3
      (Audio|Components|Audio|Play (LocalVariables|GetFootStepAudio) 0.0))))