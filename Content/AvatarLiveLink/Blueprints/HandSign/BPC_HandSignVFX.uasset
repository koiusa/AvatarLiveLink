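; Actor component that spawns particle effects at the owner's hands when the player's hand sign changes.
; On BeginPlay it caches BPC_HandSign, builds a hand pose to particle map from the HandSignVFX data table, and binds to left and right pose change events.
; OnChangePose gets hand transforms from the owner, selects the changed hand, and spawns the mapped system at that location, rotation and scale.
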(event EventBeginPlay
  (Utilities|FlowControl|Sequence
    (:then_0
      (Variables|Default|SetBPC%20Hand%20Sign (Actor|GetComponentbyClass (Components|GetOwner) "/Game/AvatarLiveLink/Blueprints/HandSign/BPC_HandSign.BPC_HandSign_C")))
    (:then_1
      (bind _output_get (Variables|Components|SetHandSignVFXDataTable "/Game/AvatarLiveLink/Blueprints/HandSign/VFX/HandSignVFX.HandSignVFX"))
      (bind _outrownames (DataTable|GetDataTableRowNames _output_get))
      (for _array_element _outrownames
        (bind _returnvalue (Utilities|GetDataTableRow (Variables|Components|GetHandSignVFXDataTable) _array_element)
          (:then
            (Utilities|Map|Add (Variables|Default|GetHandPoseVFXMap) (.HandPose (Utilities|Struct|BreakHandSignEffect _returnvalue)) (.Particle (Utilities|Struct|BreakHandSignEffect _returnvalue)))))))
    (:then_2
      (Variables|Default|GetBPC%20Hand%20Sign
        (:then
          (EventDispatchers|BindEventtoOnChengeRightPose (Variables|Default|GetBPC%20Hand%20Sign) (EventDispatchers|CreateEvent :!event OnChangePose))
          (EventDispatchers|AssignOnChangeLeftPose (Variables|Default|GetBPC%20Hand%20Sign) (EventDispatchers|CreateEvent :!event OnChangePose)))
        (:else)))))

(fn HandPoseVFX
  (params (Location :type Vector) (Rotation :type Rotator) (Scale :type Vector :default "1.000000,1.000000,1.000000") (HandPose :type HandposeIndex%20Enum :default "NewEnumerator0"))
  (Niagara|SpawnSystematLocation (.Value (Utilities|Map|Find (Variables|Default|GetHandPoseVFXMap) HandPose)) Location Rotation Scale))

(fn OnChangePose
  (params (NewPose :type Hand%20Sign%20Hand%20Pose%20Structure))
  (bind (_hand _fingers _handpose) (Utilities|Struct|BreakHandSignHandPose NewPose))
  (bind (_lefthand _righthand) (Class|BPIHandSign|GetHandTransform(Message) (Components|GetOwner)))
  (CallFunction|HandPoseVFX (.Location (Math|Transform|BreakTransform (Utilities|Select :Index _hand :NewEnumerator0 _lefthand :NewEnumerator1 _righthand))) (.Rotation (Math|Transform|BreakTransform (Utilities|Select :Index _hand :NewEnumerator0 _lefthand :NewEnumerator1 _righthand))) (.Scale (Math|Transform|BreakTransform (Utilities|Select :Index _hand :NewEnumerator0 _lefthand :NewEnumerator1 _righthand))) _handpose))