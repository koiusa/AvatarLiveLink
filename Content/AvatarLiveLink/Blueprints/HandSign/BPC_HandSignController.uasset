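; BPC_HandSignController is a controller Blueprint that toggles the player pawn's hand sign and hand sign VFX features on and off.
; Its Initialize event gets both components from player pawn 0 through getter messages and caches them.
; EnableChange flips the hand sign component's enabled flag, and VFXEnableChange independently flips the VFX component's flag.
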(event EventInitialize
  (Utilities|FlowControl|Sequence
    (:then_0
      (bind _handsignconpornent (Class|BPIHandSign|GetHandSignCompornent(Message) (Game|Player|GetPlayerPawn 0)))
      (Variables|Default|SetHandSignCompornent _handsignconpornent))
    (:then_1
      (bind _handsignvfxconpornent (Class|BPIHandSign|GetHandSignVFXCompornent(Message) (Game|Player|GetPlayerPawn 0)))
      (Variables|Default|SetHand%20Sign%20VFXConpornent _handsignvfxconpornent))))

(fn VFXEnableChange
  (bind _hand_sign_vfxconpornent (Variables|Default|GetHand%20Sign%20VFXConpornent))
  (Variables|/Game/AvatarLiveLink/Blueprints/HandSign/BPC_HandSignVFX.BPC_HandSignVFX_C|SetIsEnable _hand_sign_vfxconpornent (not (Variables|/Game/AvatarLiveLink/Blueprints/HandSign/BPC_HandSignVFX.BPC_HandSignVFX_C|GetIsEnable _hand_sign_vfxconpornent))))

(fn EnableChange
  (bind _handsigncompornent (Variables|Default|GetHandSignCompornent))
  (Variables|/Game/AvatarLiveLink/Blueprints/HandSign/BPC_HandSign.BPC_HandSign_C|SetIsEnabled _handsigncompornent (not (Variables|/Game/AvatarLiveLink/Blueprints/HandSign/BPC_HandSign.BPC_HandSign_C|GetIsEnabled _handsigncompornent))))