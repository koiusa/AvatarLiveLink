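; Blueprint function library of character and camera helpers for the AvatarLiveLink avatars.
; Respawn destroys the pawn, then passes its class and former controller to the game mode's SpawnPlayerMessage.
; Camera helpers set cine camera focus to track a character and zoom a spring arm with sign-preserving squared input, optional inversion and a minimum length.
; TrackingWeight eases a blend weight toward on or off using FInterpTo.
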(fn PlayerRespawn
  (params (Character :type Character%20Object%20Reference))
  (LocalVariables|SetControllerRef (Pawn|GetController Character))
  (Actor|DestroyActor Character)
  (Class|BPISpwaner|SpawnPlayer(Message) (Game|GetGameMode) (Utilities|GetClass Character) (LocalVariables|GetControllerRef)))

(fn SetCineCameraForcus
  (params (CineCamera :type Cine%20Camera%20Component%20Object%20Reference) (Character :type Character%20Object%20Reference))
  (Variables|/Script/CinematicCamera.CineCameraComponent|SetFocusSettings CineCamera (Utilities|Struct|MakeCameraFocusSettings "Tracking" (.manualfocusdistance (Variables|/Script/CinematicCamera.CineCameraComponent|GetFocusSettings CineCamera)) (Utilities|Struct|MakeCameraTrackingFocusSettings (Utilities|ResolveSoftReference Character) (.RelativeOffset (Utilities|Struct|BreakCameraTrackingFocusSettings (.trackingfocussettings (Variables|/Script/CinematicCamera.CineCameraComponent|GetFocusSettings CineCamera)))) (.bDrawDebugTrackingFocusPoint (Utilities|Struct|BreakCameraTrackingFocusSettings (.trackingfocussettings (Variables|/Script/CinematicCamera.CineCameraComponent|GetFocusSettings CineCamera))))) (.bsmoothfocuschanges (Variables|/Script/CinematicCamera.CineCameraComponent|GetFocusSettings CineCamera)) (.focussmoothinginterpspeed (Variables|/Script/CinematicCamera.CineCameraComponent|GetFocusSettings CineCamera)) (.focusoffset (Variables|/Script/CinematicCamera.CineCameraComponent|GetFocusSettings CineCamera))))
  (return))

(fn SetCameraZoom
  (params (SpringArm :type Spring%20Arm%20Component%20Object%20Reference) (ZoomLength :type Float%20%28single-precision%29))
  (bind _returnvalue (Math|Float|Absolute(Float) ZoomLength))
  (bind _returnvalue_2 (Math|Float|Sign(Float) ZoomLength))
  (bind _zoomspeed (LocalVariables|GetZoomSpeed))
  (bind _returnvalue_3 (Math|Float|Power _returnvalue 2.0))
  (bind _returnvalue_4 (* _returnvalue_3 _returnvalue_2))
  (bind _returnvalue_5 (* _returnvalue_4 _zoomspeed))
  (if (LocalVariables|GetInverse)
    (LocalVariables|SetTargetLength (+ (Variables|/Script/Engine.SpringArmComponent|GetTargetArmLength SpringArm) _returnvalue_5))
    (else
      (LocalVariables|SetTargetLength (- (Variables|/Script/Engine.SpringArmComponent|GetTargetArmLength SpringArm) _returnvalue_5))))
  (if (> (LocalVariables|GetTargetLength) 1e+02)
    (Variables|/Script/Engine.SpringArmComponent|SetTargetArmLength SpringArm (LocalVariables|GetTargetLength))
    (return)))

(fn TrackingWeight
  (params (IsEnable :type Boolean) (CurrentWeight :type Float%20%28single-precision%29))
  (bind _returnvalue (Utilities|Time|GetWorldDeltaSeconds))
  (bind _interpspeed (LocalVariables|GetInterpSpeed))
  (if IsEnable
    (return (Math|Interpolation|FInterpTo CurrentWeight 1.0 _returnvalue _interpspeed))
    (else
      (return (Math|Interpolation|FInterpTo CurrentWeight 0.0 _returnvalue _interpspeed)))))