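; Actor component that captures UltraLeap hand tracking on its owner and stores it in UltraLeapAdapterData.
; On BeginPlay it caches the owning Character's movement component, adds a Leap component and binds to its visibility and tracking events.
; Those events write per-hand visibility and left/right hand data into the adapter struct.
; Each tracking frame also sets IsTracking, true only while the component is enabled and the character is stationary.
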(event Custom|LeftHandVisilityChanged
  (params (bIsVisible :type Boolean))
  (Utilities|Struct|SetmembersinUltraLeapAdapterData (Variables|Default|GetUltraLeapAdapterData) bIsVisible))

(event Custom|RightHandVisilityChanged
  (params (bIsVisible :type Boolean))
  (Utilities|Struct|SetmembersinUltraLeapAdapterData (Variables|Default|GetUltraLeapAdapterData) bIsVisible))

(event Custom|OnLeapTrackingData
  (params (Frame :type Leap%20Frame%20Data%20Structure%20%28by%20ref%29))
  (bind _ultraleapadapterdata (Variables|Default|GetUltraLeapAdapterData))
  (for _array_element (.Hands (Utilities|Struct|BreakLeapFrameData Frame))
    (switch Utilities|FlowControl|Switch|SwitchonEHandType (.HandType (Utilities|Struct|BreakLeapHandData _array_element))
      (:LEAP_HAND_LEFT
        (Utilities|Struct|SetmembersinUltraLeapAdapterData _ultraleapadapterdata _array_element))
      (:LEAP_HAND_RIGHT
        (Utilities|Struct|SetmembersinUltraLeapAdapterData _ultraleapadapterdata _array_element))))
  (Utilities|Struct|SetmembersinUltraLeapAdapterData _ultraleapadapterdata (CallFunction|IsEnableTracking)))

(event EventBeginPlay
  (Utilities|FlowControl|Sequence
    (:then_0
      (bind _ascharacter (Utilities|Casting|CastToCharacter (Components|GetOwner)))
      (Variables|Default|SetCharacterMovement (Variables|/Script/Engine.Character|GetCharacterMovement _ascharacter)))
    (:then_1
      (bind _returnvalue (Game|AddComponentbyClass (Components|GetOwner) "/Script/UltraleapTracking.LeapComponent"))
      (Variables|Default|SetLeap _returnvalue)
      (EventDispatchers|BindEventtoOnLeftHandVisibilityChanged (Variables|Default|GetLeap) (EventDispatchers|CreateEvent :!event Custom|LeftHandVisilityChanged))
      (EventDispatchers|BindEventtoOnRightHandVisibilityChanged (Variables|Default|GetLeap) (EventDispatchers|CreateEvent :!event Custom|RightHandVisilityChanged))
      (EventDispatchers|BindEventtoOnLeapTrackingData (Variables|Default|GetLeap) (EventDispatchers|CreateEvent :!event Custom|OnLeapTrackingData)))))

(fn IsEnableTracking
  (return (and (not (> (Math|Vector|VectorLength (Variables|/Script/Engine.MovementComponent|GetVelocity (Variables|Default|GetCharacterMovement))) 0.0)) (Variables|Default|GetIsEnabled))))