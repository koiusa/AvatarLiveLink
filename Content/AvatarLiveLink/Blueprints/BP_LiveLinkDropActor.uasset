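; Live Link actor that swaps the player's avatar for a VRM or other model file dropped at runtime.
; Dropped files load asynchronously into a temporary asset list, scaled by extension, then OnApplyNewVRM triggers ApplyVrm.
; ApplyVrm replaces the previous MToonActor, attaches the new one to the BP_VRMTest pawn and copies poses from its source mesh through VrmAnimInstanceCopy.
; It also clears the pawn's original child avatar.
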(event Custom|LoadVrmFromFilePath
  (params (FileName :type String))
  (bind _importoption (Variables|Default|GetImportOption))
  (Utilities|FlowControl|Sequence
    (:then_0
      (bind _spawnedactor (Variables|Default|GetSpawnedActor)
        (:then
          (Actor|DestroyActor _spawnedactor))
        (:else)))
    (:then_1
      (bind _returnvalue (Game|ConstructObjectfromClass "/VRM4U/VrmAssetListObjectBP.VrmAssetListObjectBP_C" self))
      (Utilities|FlowControl|Sequence
        (:then_0
          (Utilities|Struct|SetmembersinImportOptionData _importoption (select (>= (Utilities|String|FindSubstring FileName ".vrm") 0) 1.0 0.1)))
        (:then_1
          (Variables|/Script/VRM4U.VrmAssetListObject|SetbAssetSave _returnvalue false))
        (:then_2
          (bind _outvrmasset (Class|LoaderBPFunctionLibrary|LoadVRMFileAsync _returnvalue FileName _importoption))
          ;[1 1 1] Mesh Clear
          (Class|SkinnedMeshComponent|SetSkeletalMesh (Variables|Default|GetSkeletalMesh) 0 true)
          (Default|CallOnApplyNewVRM _outvrmasset))))))

(event Custom|ApplyVrmFromAssetList
  (params (VRMAssetList :type Vrm%20Asset%20List%20Object%20Object%20Reference))
  (CallFunction|ApplyVrm VRMAssetList))

(event EventBeginPlay
  (Utilities|FlowControl|Sequence
    (:then_0
      (EventDispatchers|BindEventtoOnApplyNewVRM (delegate Custom|ApplyVrmFromAssetList)))
    (:then_1
      (EventDispatchers|AssignOnDropFiles (Variables|Default|GetVrmDropFiles) (delegate Custom|LoadVrmFromFilePath)))))

(fn ConstructionScript)

(fn ApplyVrm
  (params (VRMAssetList :type Vrm%20Asset%20List%20Object%20Object%20Reference))
  (bind _returnvalue (Game|Player|GetPlayerPawn 0))
  (bind _asbp_vrmtest (Utilities|Casting|CastToBP_VRMTest _returnvalue))
  (bind _skeletalmeshsrc (Variables|/Game/AvatarLiveLink/Blueprints/BP_VRMTest.BP_VRMTest_C|GetSkeletalMeshSrc _asbp_vrmtest))
  (Utilities|FlowControl|Sequence
    (:then_0
      (bind _spawnedactor (Variables|Default|GetSpawnedActor)
        (:then
          (Actor|DestroyActor _spawnedactor))
        (:else)))
    (:then_1
      (bind _returnvalue_2 (Game|SpawnActorfromClass "/VRM4U/Util/Actor/MToonActor.MToonActor_C" (Transformation|GetActorTransform) "Undefined" 0 VRMAssetList 5e+02 false true 0 false 0 0))
      (Variables|Default|SetSpawnedActor _returnvalue_2)
      (Utilities|FlowControl|Sequence
        (:then_0
          (Class|SkeletalMeshComponent|SetAnimClass (Variables|/VRM4U/Util/Actor/MToonActor.MToonActor_C|GetSkeletalMesh _returnvalue_2) "/Script/VRM4U.VrmAnimInstanceCopy")
          (bind _asvrm_anim_instance_copy (Utilities|Casting|CastToVrmAnimInstanceCopy (Components|SkeletalMesh|GetAnimInstance (Variables|/VRM4U/Util/Actor/MToonActor.MToonActor_C|GetSkeletalMesh _returnvalue_2))))
          (Class|VrmAnimInstanceCopy|SetSkeletalMeshCopyData _asvrm_anim_instance_copy VRMAssetList _skeletalmeshsrc 0 "/VRM4U/Util/BaseCharacter/Mesh/VRoidSimple_VrmAssetList.VRoidSimple_VrmAssetList")
          (Transformation|AttachActorToActor _returnvalue_2 _asbp_vrmtest "None" "SnapToTarget" "SnapToTarget" "SnapToTarget" true)
          (Transformation|AttachComponentToComponent (Variables|/VRM4U/Util/Actor/MToonActor.MToonActor_C|GetSkeletalMesh _returnvalue_2) _skeletalmeshsrc "None" "SnapToTarget" "SnapToTarget" "SnapToTarget" true))
        (:then_1
          (bind _childactor (Variables|/Game/AvatarLiveLink/Blueprints/BP_VRMTest.BP_VRMTest_C|GetChildActor _asbp_vrmtest)
            (:then
              (Utilities|FlowControl|Sequence
                (:then_0
                  (bind _childactor_2 (Variables|/Script/Engine.ChildActorComponent|GetChildActor _childactor)
                    (:then
                      (Actor|DestroyActor _childactor_2))
                    (:else)))
                (:then_2
                  (Components|DestroyComponent _skeletalmeshsrc))
                (:then_3
                  (Rendering|SetVisibility _skeletalmeshsrc false false))))
            (:else)))))))