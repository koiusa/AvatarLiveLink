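; Character component that feeds Live Link tracking state to an avatar through LiveLinkAdapterData.
; A runtime-added LiveLink controller drives updates for the subject picked in an on-screen selector widget.
; Each update evaluates the Basic role frame and smooths scene-frame deltas to detect whether frames still advance.
; It writes that flag and the subject to the adapter, enabling tracking only while the character stands still.
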(event Custom|OnLiveLinkUpdate
  (params (DeltaTime :type Float%20%28single-precision%29))
  (bind _subjectselecter (Variables|Default|GetSubjectSelecter))
  (Utilities|IsValid _subjectselecter
    (:Is%20Valid
      (CallFunction|UpdateLiveLinkData (Default|GetSelected _subjectselecter) DeltaTime))))

(event EventBeginPlay
  (Utilities|FlowControl|Sequence
    (:then_0
      (bind _ascharacter (Utilities|Casting|CastToCharacter (Components|GetOwner)))
      (Variables|Default|SetCharacterMovement (Variables|/Script/Engine.Character|GetCharacterMovement _ascharacter)))
    (:then_1
      (bind _returnvalue (Game|AddComponentbyClass (Components|GetOwner) "/Script/LiveLinkComponents.LiveLinkComponentController"))
      (bind _output_get (Variables|Default|SetLiveLinkController _returnvalue))
      (EventDispatchers|BindEventtoOnLiveLinkUpdated _output_get (EventDispatchers|CreateEvent :!event Custom|OnLiveLinkUpdate)))))

(fn IsEnabelTracking
  (return (== (Math|Vector|VectorLength (Variables|/Script/Engine.MovementComponent|GetVelocity (Variables|Default|GetCharacterMovement))) 0.0)))

(fn GetLiveLinkData
  (params (InputPin :type Float%20%28single-precision%29))
  (bind _returnvalue (Class|LiveLinkBlueprintLibrary|GetLiveLinkEnabledSubjectNames false))
  (if (> (Utilities|Array|Length _returnvalue) 0)
    (bind _array_element (Utilities|Array|ForEachLoopwithBreak _returnvalue :!label _label)
      (:LoopBody
        (bind _islivelinksubjectenable (CallFunction|UpdateLiveLinkData _array_element InputPin))
        (if _islivelinksubjectenable
          (goto _label Break))))
    (else
      (Utilities|Struct|SetmembersinLiveLinkAdapterData (Variables|Default|GetLiveLinkAdapterData) false false "(Name=\"\")"))))

(fn UpdateLiveLinkData
  (params (LiveLinkSubject :type Live%20Link%20Subject%20Name%20Structure) (DeltaTime :type Float%20%28double-precision%29))
  (Utilities|FlowControl|Sequence
    (:then_0
      (bind _returnvalue (Class|LiveLinkBlueprintLibrary|IsLiveLinkSubjectEnabled LiveLinkSubject))
      (if _returnvalue
        (bind _dataresult (|EvaluateLiveLinkFramewithSpecificRole LiveLinkSubject "/Script/LiveLinkInterface.LiveLinkBasicRole")
          (:then
            (Variables|Default|SetHasTrackingFrame (!= (Variables|Default|GetTImeOutCountDown) 0.0))
            (Variables|Default|SetTImeOutCountDown (Math|Interpolation|FInterpTo (Variables|Default|GetTImeOutCountDown) (- (+ (.SubFrame (Utilities|TimeManagement|BreakQualifiedFrameTime (.SceneTime (Utilities|Struct|BreakLiveLinkMetaData (.MetaData (Utilities|Struct|BreakLiveLinkBaseFrameData (.FrameData (Utilities|Struct|BreakLiveLinkBasicBlueprintData _dataresult)))))))) (Math|Conversions|ToFloat(Integer) (Utilities|Struct|BreakFrameNumber (.Frame (Utilities|TimeManagement|BreakQualifiedFrameTime (.SceneTime (Utilities|Struct|BreakLiveLinkMetaData (.MetaData (Utilities|Struct|BreakLiveLinkBaseFrameData (.FrameData (Utilities|Struct|BreakLiveLinkBasicBlueprintData _dataresult))))))))))) (Variables|Default|GetPrevFrameNumber)) DeltaTime 3e+01))
            (Variables|Default|SetPrevFrameNumber (+ (.SubFrame (Utilities|TimeManagement|BreakQualifiedFrameTime (.SceneTime (Utilities|Struct|BreakLiveLinkMetaData (.MetaData (Utilities|Struct|BreakLiveLinkBaseFrameData (.FrameData (Utilities|Struct|BreakLiveLinkBasicBlueprintData _dataresult)))))))) (Math|Conversions|ToFloat(Integer) (Utilities|Struct|BreakFrameNumber (.Frame (Utilities|TimeManagement|BreakQualifiedFrameTime (.SceneTime (Utilities|Struct|BreakLiveLinkMetaData (.MetaData (Utilities|Struct|BreakLiveLinkBaseFrameData (.FrameData (Utilities|Struct|BreakLiveLinkBasicBlueprintData _dataresult))))))))))))
            (Utilities|Struct|SetmembersinLiveLinkAdapterData (Variables|Default|GetLiveLinkAdapterData) (CallFunction|IsEnabelTracking) (Variables|Default|GetHasTrackingFrame) LiveLinkSubject))
          (:InvalidFrame
            (Variables|Default|SetPrevFrameNumber 0.0)
            (Variables|Default|SetHasTrackingFrame false)))))
    (:then_1
      (return _returnvalue (Variables|Default|GetHasTrackingFrame)))))

(fn ApplyWidget
  (params (NewParam :type Player%20Controller%20Object%20Reference))
  (bind _returnvalue (UserInterface|CreateWidget "/Game/AvatarLiveLink/Blueprints/LiveLink/WB_LiveLinkSubjects.WB_LiveLinkSubjects_C" NewParam))
  (bind _output_get (Variables|Default|SetSubjectSelecter _returnvalue))
  (UserInterface|Viewport|AddtoPlayerScreen _output_get)
  (Default|BindLiveLinkSubjects (Variables|Default|GetSubjectSelecter)))

(fn RemoveWidget
  (Widget|RemovefromParent (Variables|Default|GetSubjectSelecter))
  (Variables|Default|SetSubjectSelecter 0))